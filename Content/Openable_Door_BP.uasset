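; Door actor Blueprint that swings open and closed in response to the OnOpen and OnClose events from OpenDoor.
; The DoorSwing timeline plays forward to open and reverses to close, driving a yaw offset combined with the rotation cached at BeginPlay.
; An event track on the timeline plays the Doorlock sound at the actor's location.
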(event `self.ReceiveBeginPlay`
  (set `self.Initial Rotation` (`self.K2_GetActorRotation`)))

(event `self.OpenDoor.OnOpen`
  (bind (_direction _start_opening) (`Timeline|Door Swing` :!label _label)
    (:`Update`
      (`self.K2_SetActorRotation` (`KismetMathLibrary.ComposeRotators` (`KismetMathLibrary.MakeRotator` 0.0 0.0 _start_opening) (`self.Initial Rotation`))))
    (:`Sound event`
      (`GameplayStatics.PlaySoundAtLocation` "/Game/Audio/door-lock.door-lock" (`self.K2_GetActorLocation`)))))

(event `self.OpenDoor.OnClose`
  (goto _label :!via `Reverse`))

(fn `UserConstructionScript`)